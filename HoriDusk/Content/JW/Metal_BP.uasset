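; Metal resource Blueprint that grants metal to the player's stockpile held in the game instance.
; AddResources casts the game instance to BP_Game_Instance and increases ResourceMetal by a fixed, hard-coded amount.
; The event graph holds only disabled default events, so nothing in this Blueprint calls AddResources itself.
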(event EventBeginPlay
  (|CallParentFunction) ; This node is disabled and will not be called.\nDrag off pins to build functionality.
)

(event Collision|EventActorBeginOverlap
  (params (OtherActor :type Actor%20Object%20Reference))
  (|CallParentFunction OtherActor) ; This node is disabled and will not be called.\nDrag off pins to build functionality.
)

(event EventTick
  (params (DeltaSeconds :type Float%20%28single-precision%29))
  (|CallParentFunction DeltaSeconds) ; This node is disabled and will not be called.\nDrag off pins to build functionality.
)

(fn ConstructionScript
  (|CallParentFunction))

(fn AddResources
  (bind _asbp_game_instance (Utilities|Casting|CastToBP_Game_Instance (Game|GetGameInstance)))
  (bind _output_get (Variables|/Game/mapAssets/BP_Game_Instance.BP_Game_Instance_C|Setresource_Metal _asbp_game_instance (+ (stale _output_get) 25))))