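; Damage upgrade Blueprint that defines the name, level cap, effect text and costs for increasing the player's gun damage.
; It overrides the parent's reset to set those descriptive fields, then calls the parent version.
; Its effect value rises linearly with Level from a base amount.
; Metal and fuel costs also scale linearly, minerals join at higher levels, and all costs drop to zero at the maximum level.
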(fn ResetVirtual
  (Variables|Default|SetName "Damage")
  (Variables|Default|SetMaxLevel 8)
  (Variables|Default|SetEffect "Increase your guns' damage by 50%")
  (|CallParentFunction))

(fn GetEffectAbstract
  (return (+ (* (Variables|Default|GetLevel) 2.5) 5.0)))

(fn GetUpgradeCosts
  (bind _level (Variables|Default|GetLevel))
  (bind _returnvalue (* _level 25))
  (bind _returnvalue_2 (+ _returnvalue 25))
  (if (== _level (Variables|Default|GetMaxLevel))
    (return 0 0 0)
    (elif (< _level 4)
      (return _returnvalue_2 0 _returnvalue_2)
      (else
        (return _returnvalue_2 (+ _returnvalue -75) _returnvalue_2)))))