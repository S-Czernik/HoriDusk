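; Base Blueprint for a levelled upgrade bought with Metal, Minerals and Fuel.
; Upgrade raises Level if it is not at MaxLevel and the GameInstance holds enough resources, then deducts the cost.
; Costs and effect are placeholder functions returning zero, apparently for child overrides, and ResetVirtual zeroes Level.
; GetCostAsString uses nested selects to show only non-zero costs, displaying "Max Level" when all are zero.
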(fn GetEffectAbstract
  (return 0.0))

(fn ResetVirtual
  (Variables|Default|SetLevel 0))

(fn Upgrade
  (bind _game_instance (Variables|Default|GetGame%20Instance))
  (bind _game_instance_2 (Variables|Default|GetGame%20Instance))
  (if (not (== (Variables|Default|GetLevel) (Variables|Default|GetMaxLevel)))
    (bind (_metal_cost _mineral_cost _fuel_cost) (CallFunction|GetUpgradeCosts))
    (if (Math|Boolean|ANDBoolean (>= (- (Variables|/Game/mapAssets/BP_Game_Instance.BP_Game_Instance_C|Getresource_Metal _game_instance) _metal_cost) 0) (>= (- (Variables|/Game/mapAssets/BP_Game_Instance.BP_Game_Instance_C|Getresource_Minerals _game_instance) _mineral_cost) 0) (>= (- (Variables|/Game/mapAssets/BP_Game_Instance.BP_Game_Instance_C|Getresource_Fuel _game_instance) _fuel_cost) 0))
      (bind _output_get (Variables|Default|SetLevel (+ (stale _output_get) 1)))
      (Variables|/Game/mapAssets/BP_Game_Instance.BP_Game_Instance_C|Setresource_Metal _game_instance_2 (- (Variables|/Game/mapAssets/BP_Game_Instance.BP_Game_Instance_C|Getresource_Metal _game_instance) _metal_cost))
      (Variables|/Game/mapAssets/BP_Game_Instance.BP_Game_Instance_C|Setresource_Minerals _game_instance_2 (- (Variables|/Game/mapAssets/BP_Game_Instance.BP_Game_Instance_C|Getresource_Minerals _game_instance) _mineral_cost))
      (Variables|/Game/mapAssets/BP_Game_Instance.BP_Game_Instance_C|Setresource_Fuel _game_instance_2 (- (Variables|/Game/mapAssets/BP_Game_Instance.BP_Game_Instance_C|Getresource_Fuel _game_instance) _fuel_cost)))))

(fn GetUpgradeCosts
  (return 0 0 0))

(fn GetCostasString
  (bind (_metal_cost _mineral_cost _fuel_cost) (CallFunction|GetUpgradeCosts))
  (return (Utilities|String|SelectString "Max Level" (Utilities|String|SelectString (Utilities|String|Append "Cost: " (Utilities|String|Append "Fuel: " (Utilities|String|ToString(Integer) _fuel_cost))) (Utilities|String|SelectString (Utilities|String|Append "Cost: " (Utilities|String|Append "Minerals: " (Utilities|String|ToString(Integer) _mineral_cost))) (Utilities|String|SelectString (Utilities|String|Append "Cost: " (Utilities|String|Append "Metal: " (Utilities|String|ToString(Integer) _metal_cost))) (Utilities|String|SelectString (Utilities|String|Append (Utilities|String|Append (Utilities|String|Append "Cost: " (Utilities|String|Append "Minerals: " (Utilities|String|ToString(Integer) _mineral_cost))) ", ") (Utilities|String|Append "Fuel: " (Utilities|String|ToString(Integer) _fuel_cost))) (Utilities|String|SelectString (Utilities|String|Append (Utilities|String|Append (Utilities|String|Append "Cost: " (Utilities|String|Append "Metal: " (Utilities|String|ToString(Integer) _metal_cost))) ", ") (Utilities|String|Append "Fuel: " (Utilities|String|ToString(Integer) _fuel_cost))) (Utilities|String|SelectString (Utilities|String|Append (Utilities|String|Append (Utilities|String|Append "Cost: " (Utilities|String|Append "Metal: " (Utilities|String|ToString(Integer) _metal_cost))) ", ") (Utilities|String|Append "Minerals: " (Utilities|String|ToString(Integer) _mineral_cost))) (Utilities|String|Append (Utilities|String|Append (Utilities|String|Append (Utilities|String|Append (Utilities|String|Append "Cost: " (Utilities|String|Append "Metal: " (Utilities|String|ToString(Integer) _metal_cost))) ", ") (Utilities|String|Append "Minerals: " (Utilities|String|ToString(Integer) _mineral_cost))) ", ") (Utilities|String|Append "Fuel: " (Utilities|String|ToString(Integer) _fuel_cost))) (Math|Boolean|ANDBoolean (not (== _metal_cost 0)) (not (== _mineral_cost 0)) (== _fuel_cost 0))) (Math|Boolean|ANDBoolean (not (== _metal_cost 0)) (== _mineral_cost 0) (not (== _fuel_cost 0)))) (Math|Boolean|ANDBoolean (== _metal_cost 0) (not (== _mineral_cost 0)) (not (== _fuel_cost 0)))) (Math|Boolean|ANDBoolean (not (== _metal_cost 0)) (== _mineral_cost 0) (== _fuel_cost 0))) (Math|Boolean|ANDBoolean (== _metal_cost 0) (not (== _mineral_cost 0)) (== _fuel_cost 0))) (Math|Boolean|ANDBoolean (== _metal_cost 0) (== _mineral_cost 0) (not (== _fuel_cost 0)))) (Math|Boolean|ANDBoolean (== _metal_cost 0) (== _mineral_cost 0) (== _fuel_cost 0)))))