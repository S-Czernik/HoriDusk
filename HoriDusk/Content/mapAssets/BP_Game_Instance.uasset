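; Game instance Blueprint that holds run state: player upgrade levels, map seed and map-generated flag.
; On Init it calls RestartGame, which zeroes the health, fire-rate and gun-damage upgrades, picks a random seed, resets SeedLast and clears MapGenerated.
; Three getter graphs contain upgrade scaling formulas for damage, fire rate and exponential max health, but those nodes appear unconnected.
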(event EventInit
  (CallFunction|RestartGame))

(fn RestartGame
  (CallFunction|RestartUpgrades)
  (Variables|Default|Setseed (Math|Random|RandomInteger 999999))
  (Variables|Default|SetseedLast (Variables|Default|GetseedFirstFirst))
  (Variables|Default|SetmapGenerated false))

(fn RestartUpgrades
  (Variables|Default|Setupgrade_MaxHealth 0)
  (Variables|Default|Setupgrade_FireRate 0)
  (Variables|Default|Setupgrade_GunDamage 0))