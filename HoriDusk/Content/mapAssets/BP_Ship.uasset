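; BP_Ship is the map ship that flies in a straight line to a target position set by MoveTo.
; Once the game instance reports the map generated, Tick creates the main UI and teleports the ship above TargetPlanet.
; While travelling it moves at constant speed, but burns Fuel and advances BP_Clock per frame.
; Within tolerance it snaps to the target, sets Landed and clears the game instance's PlanetRef.
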(event EventTick
  (params (DeltaSeconds :type Float%20%28single-precision%29))
  (bind _returnvalue (Transformation|GetActorLocation))
  (bind _targetplanet (Variables|Default|GettargetPlanet))
  (bind _returnvalue_2 (Transformation|GetActorLocation _targetplanet))
  (bind _returnvalue_3 (+ _returnvalue_2 "0.000000,0.000000,100.000000"))
  (if (Variables|Default|GetshipSpawned)
    ;[1 1 1] Calculate Position
    (if (Utilities|Operators|EqualEqual _returnvalue (Variables|Default|GetTargetPosition) 5e+01)
      (Transformation|SetActorLocation (Variables|Default|GetTargetPosition) false false)
      (Variables|Default|Setlanded true)
      (bind _asbp_game_instance (Utilities|Casting|CastToBP_Game_Instance (Game|GetGameInstance)))
      (Variables|/Game/mapAssets/BP_Game_Instance.BP_Game_Instance_C|SetplanetRef _asbp_game_instance 0)
      (else
        (Variables|Default|Setlanded false)
        (Transformation|SetActorLocation (- _returnvalue (* (* (Math|Vector|Normalize (- _returnvalue (Variables|Default|GetTargetPosition))) DeltaSeconds) "500.000000,500.000000,500.000000")) false false)
        (bind _outactors (Actor|GetAllActorsOfClass "/Game/mapAssets/BP_Clock.BP_Clock_C"))
        (bind _newparam (Default|GetTimeElapsed _outactors))
        (Default|SetTimeElapsed _outactors (+ _newparam 80))
        (Variables|Default|SetFuel (- (Variables|Default|GetFuel) 1.0))))
    (else
      (bind _asbp_game_instance_2 (Utilities|Casting|CastToBP_Game_Instance (Game|GetGameInstance)))
      (if (Variables|/Game/mapAssets/BP_Game_Instance.BP_Game_Instance_C|GetmapGenerated _asbp_game_instance_2)
        ;[1 1 1] Default Position
        (bind _returnvalue_4 (UserInterface|CreateWidget "/Game/mapAssets/BP_Main_UI.BP_Main_UI_C"))
        (UserInterface|Viewport|AddtoViewport _returnvalue_4 0)
        (Variables|Default|SetTargetPosition _returnvalue_3)
        (Transformation|SetActorLocation _returnvalue_3 false true)
        (Variables|Default|SetshipSpawned true)))))

(fn ConstructionScript)

(fn Moveto
  (params (ToPosition :type Vector))
  (Variables|Default|SetTargetPosition ToPosition))