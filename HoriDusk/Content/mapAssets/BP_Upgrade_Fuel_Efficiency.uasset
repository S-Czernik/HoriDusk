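; BP_Upgrade_Fuel_Efficiency is a ship upgrade that raises fuel efficiency by a fixed step per level.
; It overrides the parent's reset to set its name, level cap and description text, then calls the parent implementation.
; The effect is a multiplier that grows linearly with level.
; Metal, mineral and fuel costs are equal, rise piecewise-linearly in three steepening tiers, and return zero at max level.
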(fn ResetVirtual
  (Variables|Default|SetName "Fuel Efficiecy")
  (Variables|Default|SetMaxLevel 12)
  (Variables|Default|SetEffect "Increase your ship's fuel efficiency by 20%")
  (|CallParentFunction))

(fn GetEffectAbstract
  (return (+ (* (Variables|Default|GetLevel) 0.2) 1.0)))

(fn GetUpgradeCosts
  (bind _level (Variables|Default|GetLevel))
  (bind _returnvalue (* _level 25))
  (bind _returnvalue_2 (* _level 100))
  (bind _returnvalue_3 (* _level 50))
  (bind _returnvalue_4 (+ _returnvalue_3 -50))
  (bind _returnvalue_5 (+ _returnvalue 25))
  (bind _returnvalue_6 (+ _returnvalue_2 -400))
  (if (== _level (Variables|Default|GetMaxLevel))
    (return 0 0 0)
    (elif (< _level 4)
      (return _returnvalue_5 _returnvalue_5 _returnvalue_5)
      (elif (< _level 8)
        (return _returnvalue_4 _returnvalue_4 _returnvalue_4)
        (else
          (return _returnvalue_6 _returnvalue_6 _returnvalue_6))))))