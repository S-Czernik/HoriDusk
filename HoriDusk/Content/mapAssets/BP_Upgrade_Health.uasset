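; Health upgrade Blueprint that raises maximum health by 50 per level from a base of 100, up to level 8.
; It overrides a parent upgrade's reset, effect and cost functions to supply its name, level cap, description, effect value and prices.
; Costs scale with level, using only metal for early levels, adding minerals from level 4 and dropping to zero at max level.
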(fn ResetVirtual
  (Variables|Default|SetName "Health")
  (Variables|Default|SetMaxLevel 8)
  (Variables|Default|SetEffect "Increase your maximum health by 50")
  (|CallParentFunction))

(fn GetEffectAbstract
  (return (Math|Conversions|ToFloat(Integer) (+ (* (Variables|Default|GetLevel) 50) 100))))

(fn GetUpgradeCosts
  (bind _level (Variables|Default|GetLevel))
  (bind _returnvalue (* _level 50))
  (if (== _level (Variables|Default|GetMaxLevel))
    (return 0 0 0)
    (elif (< _level 4)
      (return (+ (* _level 25) 25) 0 0)
      (else
        (return (+ _returnvalue -50) (+ _returnvalue -150) 0)))))