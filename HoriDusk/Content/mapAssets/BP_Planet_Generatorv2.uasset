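; Map generator actor that spawns a seeded field of planets on BeginPlay, plus a start planet and a target planet offset by the path length.
; A seed-driven modular recurrence from the game instance sets planet count and positions, storing its last value back.
; Later generations restore landability from visited flags and mark planets progressively nearer the saved ship position as visited.
; The ship is then targeted at the closest match.
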(event EventBeginPlay
  (bind _self self)
  (bind _returnvalue (Transformation|GetActorLocation _self))
  (bind _asbp_game_instance (Utilities|Casting|CastToBP_Game_Instance (Game|GetGameInstance)))
  (Variables|Default|SetAs%20BP%20Game%20Instance _asbp_game_instance)
  (bind _outactors (Actor|GetAllActorsOfClass "/Game/mapAssets/BP_Ship.BP_Ship_C"))
  (for _array_element _outactors
    (Variables|Default|SetshipRef _array_element))
  (bind _returnvalue_2 (Game|SpawnActorfromClass "/Game/mapAssets/BP_Planet.BP_Planet_C" (Math|Conversions|ToTransform(Vector) _returnvalue) "AdjustIfPossibleButAlwaysSpawn" "MultiplyWithRoot" 0 0))
  (Variables|Default|SetfirstPlanet _returnvalue_2)
  ;[1 1 1] Spawning planets based on seed
  (bind _result (Math|Float|NegateFloat (Variables|Default|GetPath%20Length))
    (:%20%20
      (Game|SpawnActorfromClass "/Game/mapAssets/BP_Target_Planet.BP_Target_Planet_C" (Math|Conversions|ToTransform(Vector) (+ _returnvalue (Math|Vector|MakeVector _result 0.0 0.0))) "AdjustIfPossibleButAlwaysSpawn" "MultiplyWithRoot" 0 0)
      (bind _asbp_game_instance_2 (Utilities|Casting|CastToBP_Game_Instance (Game|GetGameInstance)))
      (Variables|Default|SetAs%20BP%20Game%20Instance _asbp_game_instance_2)
      (Variables|Default|SetlastNumber (Variables|/Game/mapAssets/BP_Game_Instance.BP_Game_Instance_C|GetseedLast _asbp_game_instance_2))
      (for _index (range 0 (+ (Math|Integer|%(Integer) (Variables|/Game/mapAssets/BP_Game_Instance.BP_Game_Instance_C|Getseed _asbp_game_instance) 20) 20))
        (bind _output_get (Variables|Default|SetlastNumber (+ (Math|Integer|%(Integer) (* (+ (Variables|/Game/mapAssets/BP_Game_Instance.BP_Game_Instance_C|Getseed (Variables|Default|GetAs%20BP%20Game%20Instance)) 8000) (Variables|Default|GetlastNumber)) 999999) (Variables|/Game/mapAssets/BP_Game_Instance.BP_Game_Instance_C|GetseedA (Variables|Default|GetAs%20BP%20Game%20Instance)))))
        (bind _result_2 (Math|Float|NegateFloat (Math|Float|%(Float) (Math|Conversions|ToFloat(Integer) (* (+ (Variables|/Game/mapAssets/BP_Game_Instance.BP_Game_Instance_C|Getseed (Variables|Default|GetAs%20BP%20Game%20Instance)) 8000) (Variables|Default|GetlastNumber))) (Variables|Default|GetPath%20Length)))
          (:%20%20
            (bind _output_get_2 (Variables|Default|SettempX (Math|Float|Truncate _result_2)))
            (bind _output_get_3 (Variables|Default|SetlastNumber (+ (Math|Integer|%(Integer) (* (+ (Variables|/Game/mapAssets/BP_Game_Instance.BP_Game_Instance_C|Getseed (Variables|Default|GetAs%20BP%20Game%20Instance)) 8000) _output_get) 999999) (Variables|/Game/mapAssets/BP_Game_Instance.BP_Game_Instance_C|GetseedA (Variables|Default|GetAs%20BP%20Game%20Instance)))))
            (bind _output_get_4 (Variables|Default|SettempY (Math|Float|Truncate (- (Math|Float|%(Float) (Math|Conversions|ToFloat(Integer) (* (+ (Variables|/Game/mapAssets/BP_Game_Instance.BP_Game_Instance_C|Getseed (Variables|Default|GetAs%20BP%20Game%20Instance)) 8000) _output_get)) 5e+02) 2.5e+02))))
            (Variables|Default|SetlastNumber (+ (Math|Integer|%(Integer) (* (+ (Variables|/Game/mapAssets/BP_Game_Instance.BP_Game_Instance_C|Getseed (Variables|Default|GetAs%20BP%20Game%20Instance)) 8000) _output_get_3) 999999) (Variables|/Game/mapAssets/BP_Game_Instance.BP_Game_Instance_C|GetseedA (Variables|Default|GetAs%20BP%20Game%20Instance))))
            (bind _output_get_5 (Variables|Default|SettempZ (Math|Float|Truncate (+ (Math|Float|%(Float) (Math|Conversions|ToFloat(Integer) (* (+ (Variables|/Game/mapAssets/BP_Game_Instance.BP_Game_Instance_C|Getseed (Variables|Default|GetAs%20BP%20Game%20Instance)) 8000) _output_get_3)) 1e+02) 3e+02))))
            (bind _output_get_6 (Variables|Default|SetnewTrans (Math|Conversions|ToTransform(Vector) (Math|Vector|MakeVector (Math|Conversions|ToFloat(Integer) _output_get_2) (Math|Conversions|ToFloat(Integer) _output_get_4) (Math|Conversions|ToFloat(Integer) _output_get_5)))))
            (bind _returnvalue_3 (Game|SpawnActorfromClass "/Game/mapAssets/BP_Planet.BP_Planet_C" _output_get_6 "AdjustIfPossibleButAlwaysSpawn" "MultiplyWithRoot" 0 0))
            (Variables|/Game/mapAssets/BP_Planet.BP_Planet_C|Setid _returnvalue_3 (Variables|Default|Geti))
            (Variables|Default|Seti (+ (Variables|Default|Geti) 1))
            (if (Variables|/Game/mapAssets/BP_Game_Instance.BP_Game_Instance_C|GetfirstGeneration (Variables|Default|GetAs%20BP%20Game%20Instance))
              (Utilities|Array|Add (Variables|/Game/mapAssets/BP_Game_Instance.BP_Game_Instance_C|GetplanetsVisited (Variables|Default|GetAs%20BP%20Game%20Instance)) false)
              (else
                ;[1 1 1] only on another generation
                (Variables|/Game/mapAssets/BP_Planet.BP_Planet_C|Setlandable _returnvalue_3 (not (Utilities|Array|Get(acopy) (Variables|/Game/mapAssets/BP_Game_Instance.BP_Game_Instance_C|GetplanetsVisited (Variables|Default|GetAs%20BP%20Game%20Instance)) (Variables|Default|Geti))))
                ;;[1 1 1] player ship planet
                (if (> (Variables|Default|Getdistance) (+ (Math|Float|Power (.x (- (Transformation|GetActorLocation _returnvalue_3) (Variables|/Game/mapAssets/BP_Game_Instance.BP_Game_Instance_C|GetshipPosition (Variables|Default|GetAs%20BP%20Game%20Instance)))) 2.0) (Math|Float|Power (.y (- (Transformation|GetActorLocation _returnvalue_3) (Variables|/Game/mapAssets/BP_Game_Instance.BP_Game_Instance_C|GetshipPosition (Variables|Default|GetAs%20BP%20Game%20Instance)))) 2.0) (Math|Float|Power (.z (- (Transformation|GetActorLocation _returnvalue_3) (Variables|/Game/mapAssets/BP_Game_Instance.BP_Game_Instance_C|GetshipPosition (Variables|Default|GetAs%20BP%20Game%20Instance)))) 2.0)))
                  (Utilities|Array|SetArrayElem (Variables|/Game/mapAssets/BP_Game_Instance.BP_Game_Instance_C|GetplanetsVisited (Variables|Default|GetAs%20BP%20Game%20Instance)) (Variables|Default|Geti) true)
                  (Variables|Default|Setdistance (+ (Math|Float|Power (.x (- (Transformation|GetActorLocation _returnvalue_3) (Variables|/Game/mapAssets/BP_Game_Instance.BP_Game_Instance_C|GetshipPosition (Variables|Default|GetAs%20BP%20Game%20Instance)))) 2.0) (Math|Float|Power (.y (- (Transformation|GetActorLocation _returnvalue_3) (Variables|/Game/mapAssets/BP_Game_Instance.BP_Game_Instance_C|GetshipPosition (Variables|Default|GetAs%20BP%20Game%20Instance)))) 2.0) (Math|Float|Power (.z (- (Transformation|GetActorLocation _returnvalue_3) (Variables|/Game/mapAssets/BP_Game_Instance.BP_Game_Instance_C|GetshipPosition (Variables|Default|GetAs%20BP%20Game%20Instance)))) 2.0)))
                  (Variables|Default|SetfirstPlanet _returnvalue_3)
                  (Variables|/Game/mapAssets/BP_Planet.BP_Planet_C|Setlandable _returnvalue_3 false)))))))
      (bind _asbp_game_instance_3 (Utilities|Casting|CastToBP_Game_Instance (Game|GetGameInstance)))
      (Variables|/Game/mapAssets/BP_Game_Instance.BP_Game_Instance_C|SetseedLast _asbp_game_instance_3 (Variables|Default|GetlastNumber))
      ;;[1 0.03957 0.6258] ship starting position
      (Variables|/Game/mapAssets/BP_Ship.BP_Ship_C|SettargetPlanet (Variables|Default|GetshipRef) (Variables|Default|GetfirstPlanet))
      (Variables|/Game/mapAssets/BP_Ship.BP_Ship_C|SetTargetPosition (Variables|Default|GetshipRef) (Transformation|GetActorLocation (Variables|Default|GetfirstPlanet)))
      (Variables|/Game/mapAssets/BP_Game_Instance.BP_Game_Instance_C|SetmapGenerated _asbp_game_instance_3 true)
      (Variables|/Game/mapAssets/BP_Game_Instance.BP_Game_Instance_C|SetfirstGeneration _asbp_game_instance_3 false))))

(event Collision|EventActorBeginOverlap
  (params (OtherActor :type Actor%20Object%20Reference)))

(event EventTick
  (params (DeltaSeconds :type Float%20%28single-precision%29)))

(fn ConstructionScript)

(fn NewFunction)