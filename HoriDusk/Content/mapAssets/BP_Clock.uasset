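; BP_Clock is a game clock that counts elapsed time and mirrors it into BP_Game_Instance.
; On Tick it waits for the game instance's MapGenerated flag, then restores the saved TimeElapsed once.
; While switched on, it accumulates delta time scaled by the instance's ClockSpeed, moving whole units into TimeElapsed and carrying the fraction over.
; Run, stop, get and set functions control it.
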(event EventTick
  (params (DeltaSeconds :type Float%20%28single-precision%29))
  (if (Variables|Default|GetclockSpawned)
    (if (Variables|Default|GetclockOn)
      (if (> (Variables|Default|GetcutTime) 1.0)
        (Variables|Default|SettimeToIncrement (Math|Float|Floor (Variables|Default|GetcutTime)))
        (Variables|Default|SetcutTime (- (Variables|Default|GetcutTime) (Variables|Default|GettimeToIncrement)))
        (CallFunction|SetTimeElapsed (+ (Variables|Default|GettimeElapsed) (Variables|Default|GettimeToIncrement)))
        (Variables|Default|SettimeToIncrement 0)
        (bind _asbp_game_instance (Utilities|Casting|CastToBP_Game_Instance (Game|GetGameInstance)))
        (Variables|/Game/mapAssets/BP_Game_Instance.BP_Game_Instance_C|SettimeElapsed _asbp_game_instance (Variables|Default|GettimeElapsed))
        (else
          (bind _asbp_game_instance_2 (Utilities|Casting|CastToBP_Game_Instance (Game|GetGameInstance)))
          (Variables|Default|SetcutTime (+ (Variables|Default|GetcutTime) (* DeltaSeconds (Variables|/Game/mapAssets/BP_Game_Instance.BP_Game_Instance_C|GetclockSpeed _asbp_game_instance_2)))))))
    (else
      (bind _asbp_game_instance_3 (Utilities|Casting|CastToBP_Game_Instance (Game|GetGameInstance)))
      (if (Variables|/Game/mapAssets/BP_Game_Instance.BP_Game_Instance_C|GetmapGenerated _asbp_game_instance_3)
        (Variables|Default|SettimeElapsed (Variables|/Game/mapAssets/BP_Game_Instance.BP_Game_Instance_C|GettimeElapsed _asbp_game_instance_3))
        (Variables|Default|SetclockSpawned true)))))

(fn ConstructionScript)

(fn SetTimeElapsed
  (params (timeElapsed :type Integer))
  (Variables|Default|SettimeElapsed timeElapsed))

(fn GetTimeElapsed
  (return (Variables|Default|GettimeElapsed)))

(fn RunClock
  (Variables|Default|SetclockOn true))

(fn StopClock
  (Variables|Default|SetclockOn false))