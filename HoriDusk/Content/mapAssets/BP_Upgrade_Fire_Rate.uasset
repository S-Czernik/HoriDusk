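; Fire Rate upgrade Blueprint that boosts the firerate of guns across four levels.
; It overrides a parent upgrade's reset to set its name, level cap and description, and returns a multiplier that grows linearly by a quarter per level.
; Costs come in equal metal and mineral with no fuel, rise more steeply at higher levels, and drop to zero at max level.
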(fn ResetVirtual
  (Variables|Default|SetName "Fire Rate")
  (Variables|Default|SetMaxLevel 4)
  (Variables|Default|SetEffect "Increase your guns' firerate by 25%")
  (|CallParentFunction))

(fn GetEffectAbstract
  (return (+ (* (Variables|Default|GetLevel) 0.25) 1.0)))

(fn GetUpgradeCosts
  (bind _level (Variables|Default|GetLevel))
  (bind _returnvalue (* _level 25))
  (bind _returnvalue_2 (* _level 100))
  (bind _returnvalue_3 (+ _returnvalue 25))
  (bind _returnvalue_4 (+ _returnvalue_2 -100))
  (if (== _level (Variables|Default|GetMaxLevel))
    (return 0 0 0)
    (elif (< _level 2)
      (return _returnvalue_3 _returnvalue_3 0)
      (else
        (return _returnvalue_4 _returnvalue_4 0)))))