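; BP_Turret is an enemy turret that turns to face the player and fires bullets.
; When PawnSensing sees the player character, the actor snaps its rotation toward the player's location.
; After a short delay it spawns BP_MyBullet at the Arrow component's transform.
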(event OnSeePawn(PawnSensing)
  (params (Pawn :type Pawn%20Object%20Reference))
  (Utilities|Casting|CastToPlayerCharacter Pawn)
  (Transformation|SetActorRotation (Math|Conversions|RotationFromXVector (.X (Math|Rotator|GetAxes (Math|Rotator|FindLookatRotation (Transformation|GetActorLocation) (Transformation|GetActorLocation Pawn))))))
  (Utilities|FlowControl|Delay 0.2)
  (Game|SpawnActorfromClass "/Game/FirstPerson/Blueprints/BP_MyBullet.BP_MyBullet_C" (Transformation|GetWorldTransform (Variables|Default|GetArrow)) "Undefined" "MultiplyWithRoot" 0 0))

(fn ConstructionScript)