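; Boss turret that aims at the player with random error and fires BP_MyBossBullet1 from two arrow components.
; Tick drives aiming and, through a 0.75-second Delay, paired shots with slight random jitter, also caching the last TerrainBP found.
; DealDamage subtracts the player's AttackPower from clamped HP.
; At zero HP, Death fades the camera, destroys player and turret, and shows an end-screen widget (WB_Death_UI1, stored as Winui).
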(event Custom|Death
  (CameraFades|StartCameraFade :self (Game|GetPlayerCameraManager 0) :ToAlpha 1.0 :Duration 5.0 :bHoldWhenFinished true)
  (Utilities|FlowControl|Delay 5.0)
  (Actor|DestroyActor (Game|Player|GetPlayerPawn 0))
  (Variables|/Script/Engine.PlayerController|SetbShowMouseCursor (Game|GetPlayerController 0) true)
  (bind _returnvalue (UserInterface|CreateWidget "/Game/FirstPerson/UI/WB_Death_UI1.WB_Death_UI1_C"))
  (bind _output_get (Variables|Default|SetWinui _returnvalue))
  (UserInterface|Viewport|AddtoViewport _output_get 0)
  (Actor|DestroyActor))

(event Custom|Deal%20Damage
  ;[1 1 1] Updating HP when damaged
  (bind _asplayer_character (Utilities|Casting|CastToPlayerCharacter (Game|Player|GetPlayerPawn 0)))
  (if (not (Variables|Default|GetDead))
    (bind _output_get (Variables|Default|SetCurrent_HP (Math|Float|Clamp(Float) (- (Variables|Default|GetCurrent_HP) (Variables|/Game/FirstPerson/Blueprints/PlayerCharacter.PlayerCharacter_C|GetAttack_Power _asplayer_character)) 0.0 (Variables|Default|GetMax_HP))))
    (if (== _output_get 0.0)
      (CallFunction|Death))))

(event EventTick
  (params (DeltaSeconds :type Float%20%28single-precision%29))
  (bind _returnvalue (Math|Random|RandomUnitVector))
  (bind _arrow3 (Variables|Default|GetArrow3))
  (bind _arrow (Variables|Default|GetArrow))
  (bind _returnvalue_2 (Transformation|GetWorldTransform _arrow3))
  (bind _returnvalue_3 (Transformation|GetWorldTransform _arrow))
  (Variables|Default|SetNewVar (Math|Vector|MakeVector (Math|Float|%(Float) (.x _returnvalue) 8e+01) (Math|Float|%(Float) (.y _returnvalue) 8e+01) (Math|Float|%(Float) (.z _returnvalue) 8e+01)))
  ;[1 1 1] Seek and attack player
  (bind _outactors (Actor|GetAllActorsOfClass "/Game/FirstPerson/Blueprints/PlayerCharacter.PlayerCharacter_C"))
  (Transformation|SetActorRotation (Math|Rotator|FindLookatRotation (Transformation|GetActorLocation) (+ (Transformation|GetActorLocation (Utilities|Array|Get(acopy) _outactors)) (* (Math|Random|RandomUnitVector) (Variables|Default|GetError_Multiplier)))))
  (Utilities|FlowControl|Delay 0.75)
  (Game|SpawnActorfromClass "/Game/FirstPerson/Blueprints/BP_MyBossBullet1.BP_MyBossBullet1_C" (Math|Transform|MakeTransform (+ (Math|Vector|MakeVector (.x (Variables|Default|GetNewVar)) (.y (Variables|Default|GetNewVar)) (.z (Variables|Default|GetNewVar))) (.location _returnvalue_3)) (Math|Rotator|MakeRotator (+ (.x (Variables|Default|GetNewVar)) (.roll (.rotation _returnvalue_3))) (+ (.y (Variables|Default|GetNewVar)) (.pitch (.rotation _returnvalue_3))) (+ (.z (Variables|Default|GetNewVar)) (.yaw (.rotation _returnvalue_3)))) (.scale _returnvalue_3)) "Undefined" "MultiplyWithRoot" 0 0)
  (bind _outactors_2 (Actor|GetAllActorsOfClass "/Game/JW/TerrainBP.TerrainBP_C"))
  (for _array_element _outactors_2
    (Variables|Default|Setterrain _array_element))
  (Game|SpawnActorfromClass "/Game/FirstPerson/Blueprints/BP_MyBossBullet1.BP_MyBossBullet1_C" (Math|Transform|MakeTransform (+ (Math|Vector|MakeVector (.x (Variables|Default|GetNewVar)) (.y (Variables|Default|GetNewVar)) (.z (Variables|Default|GetNewVar))) (.location _returnvalue_2)) (Math|Rotator|MakeRotator (+ (.x (Variables|Default|GetNewVar)) (.roll (.rotation _returnvalue_2))) (+ (.y (Variables|Default|GetNewVar)) (.pitch (.rotation _returnvalue_2))) (+ (.z (Variables|Default|GetNewVar)) (.yaw (.rotation _returnvalue_2)))) (.scale _returnvalue_2)) "Undefined" "MultiplyWithRoot" 0 0)
  (bind _outactors_3 (Actor|GetAllActorsOfClass "/Game/JW/TerrainBP.TerrainBP_C"))
  (for _array_element_2 _outactors_3
    (Variables|Default|Setterrain _array_element_2)))

(fn ConstructionScript)