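; Clickable map planet that serves as a travel destination for BP_Ship and rolls random Fuel, Metal and Minerals levels in its construction script.
; Clicking while the ship is landed resets all planets' materials, highlights this one and moves the ship above it.
; Tick shows the selection widget, turns both widgets toward the camera and pushes resource levels into the details widget, which appears on hover.
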(event OnBeginCursorOver(sphereComponent)
  (params (TouchedComponent :type Primitive%20Component%20Object%20Reference))
  ;[1 1 1] UI Details toggle
  (Rendering|SetVisibility (Variables|Default|GetDetailsWidget) true true))

(event OnClicked(sphereComponent)
  (params (TouchedComponent :type Primitive%20Component%20Object%20Reference) (ButtonPressed :type Key%20Structure :default "None"))
  (bind _asbp_ship (Utilities|Casting|CastToBP_Ship (Variables|Default|GetshipRef)))
  (if (Variables|/Game/mapAssets/BP_Ship.BP_Ship_C|Getlanded _asbp_ship)
    (CallFunction|OnClickonSelf)
    (Variables|Default|Setselected true)
    (CallFunction|CalltoShip)))

(event OnEndCursorOver(sphereComponent)
  (params (TouchedComponent :type Primitive%20Component%20Object%20Reference))
  ;[1 1 1] UI Details toggle
  (Rendering|SetVisibility (Variables|Default|GetDetailsWidget) false true))

(event EventTick
  (params (DeltaSeconds :type Float%20%28single-precision%29))
  (bind _returnvalue (Game|GetPlayerCameraManager 0))
  (bind _detailswidget (Variables|Default|GetDetailsWidget))
  (bind _returnvalue_2 (Transformation|GetWorldLocation _detailswidget))
  (bind _transformcomponent (Variables|/Script/Engine.PlayerCameraManager|GetTransformComponent _returnvalue))
  (bind _returnvalue_3 (Transformation|GetWorldLocation _transformcomponent))
  (bind _returnvalue_4 (Math|Rotator|FindLookatRotation _returnvalue_2 _returnvalue_3))
  (Utilities|FlowControl|Sequence
    (:then_0
      (if (Variables|Default|Getselected)
        (if (Variables|Default|GethasWidget)
          (Transformation|SetWorldRotation (Variables|Actor|GetWidget) (Math|Rotator|FindLookatRotation (Transformation|GetWorldLocation (Variables|Actor|GetWidget)) (Transformation|GetWorldLocation (Variables|/Script/Engine.PlayerCameraManager|GetTransformComponent (Game|GetPlayerCameraManager 0)))) false false)
          (else
            (Rendering|SetVisibility (Variables|Actor|GetWidget) true false)
            (Variables|Default|SethasWidget true)))
        (elif (Variables|Default|GethasWidget)
          (Rendering|SetVisibility (Variables|Actor|GetWidget) false false)
          (Variables|Default|SethasWidget false))))
    (:then_1
      (Transformation|SetWorldRotation (Variables|Default|GetDetailsWidget) (Math|Rotator|MakeRotator (.roll _returnvalue_4) 0.0 (.yaw _returnvalue_4)) false false))
    (:then_2
      (bind _asbp_planet_details (Utilities|Casting|CastToBP_Planet_Details (UserInterface|GetUserWidgetObject (Variables|Default|GetDetailsWidget))))
      (switch Utilities|FlowControl|Switch|SwitchonResources (Variables|Default|GetFuel)
        (:NewEnumerator0
          (Variables|/Game/mapAssets/BP_Planet_Details.BP_Planet_Details_C|SetfuelValue _asbp_planet_details "High"))
        (:NewEnumerator1
          (Variables|/Game/mapAssets/BP_Planet_Details.BP_Planet_Details_C|SetfuelValue _asbp_planet_details "Medium"))
        (:NewEnumerator2
          (Variables|/Game/mapAssets/BP_Planet_Details.BP_Planet_Details_C|SetfuelValue _asbp_planet_details "Low"))
        (:NewEnumerator3
          (Variables|/Game/mapAssets/BP_Planet_Details.BP_Planet_Details_C|SetfuelValue _asbp_planet_details "None")))
      (switch Utilities|FlowControl|Switch|SwitchonResources (Variables|Default|GetMinerals)
        (:NewEnumerator0
          (Variables|/Game/mapAssets/BP_Planet_Details.BP_Planet_Details_C|SetmineralsValue _asbp_planet_details "High"))
        (:NewEnumerator1
          (Variables|/Game/mapAssets/BP_Planet_Details.BP_Planet_Details_C|SetmineralsValue _asbp_planet_details "Medium"))
        (:NewEnumerator2
          (Variables|/Game/mapAssets/BP_Planet_Details.BP_Planet_Details_C|SetmineralsValue _asbp_planet_details "Low"))
        (:NewEnumerator3
          (Variables|/Game/mapAssets/BP_Planet_Details.BP_Planet_Details_C|SetmineralsValue _asbp_planet_details "None")))
      (switch Utilities|FlowControl|Switch|SwitchonResources (Variables|Default|GetMetal)
        (:NewEnumerator0
          (Variables|/Game/mapAssets/BP_Planet_Details.BP_Planet_Details_C|SetmetalValue _asbp_planet_details "High"))
        (:NewEnumerator1
          (Variables|/Game/mapAssets/BP_Planet_Details.BP_Planet_Details_C|SetmetalValue _asbp_planet_details "Medium"))
        (:NewEnumerator2
          (Variables|/Game/mapAssets/BP_Planet_Details.BP_Planet_Details_C|SetmetalValue _asbp_planet_details "Low"))
        (:NewEnumerator3
          (Variables|/Game/mapAssets/BP_Planet_Details.BP_Planet_Details_C|SetmetalValue _asbp_planet_details "None"))))))

(event EventBeginPlay
  (Variables|/Script/Engine.PlayerController|SetbEnableMouseOverEvents (Game|GetPlayerController 0) true))

(fn ConstructionScript
  (bind _outactors (Actor|GetAllActorsOfClass "/Game/mapAssets/BP_Ship.BP_Ship_C"))
  (Variables|Default|SetshipRef (.ReturnValue (Actor|FindNearestActor "0, 0, 0" _outactors)))
  (Variables|Default|SetFuel (.OutItem (Utilities|Array|Random (Variables|Default|GetenumArray))))
  (Variables|Default|SetMetal (.OutItem (Utilities|Array|Random (Variables|Default|GetenumArray))))
  (Variables|Default|SetMinerals (.OutItem (Utilities|Array|Random (Variables|Default|GetenumArray)))))

(fn OnClickonSelf
  (bind _outactors (Actor|GetAllActorsOfClass "BP_Planet_C"))
  (bind _outactors_2 (Actor|GetAllActorsOfClass "/Game/mapAssets/BP_Target_Planet.BP_Target_Planet_C"))
  (for _array_element _outactors
    (if (Actor|ActorHasTag _array_element "Target")
      (Rendering|Material|SetMaterial (Variables|BP_Planet_C|GetsphereComponent _array_element) 0 "/Game/StarterContent/Materials/M_Water_Ocean.M_Water_Ocean")
      (Variables|BP_Planet_C|Setselected _array_element false)
      (else
        (Rendering|Material|SetMaterial (Variables|BP_Planet_C|GetsphereComponent _array_element) 0 "/Game/StarterContent/Materials/M_Rock_Sandstone.M_Rock_Sandstone")
        (Variables|BP_Planet_C|Setselected _array_element false))))
  (for _array_element_2 _outactors_2
    (Rendering|Material|SetMaterial (Variables|/Game/mapAssets/BP_Target_Planet.BP_Target_Planet_C|GetsphereComponent _array_element_2) 0 "/Game/StarterContent/Materials/M_Water_Ocean.M_Water_Ocean")
    (Variables|Default|Setselected false))
  (return))

(fn CalltoShip
  (bind _returnvalue (Transformation|GetActorLocation))
  (Rendering|Material|SetMaterial (Variables|Default|GetsphereComponent) 0 "/Game/StarterContent/Materials/M_CobbleStone_Smooth.M_CobbleStone_Smooth")
  (bind _asbp_ship (Utilities|Casting|CastToBP_Ship (Variables|Default|GetshipRef)))
  (Rendering|Material|SetMaterial (Variables|/Game/mapAssets/BP_Ship.BP_Ship_C|GetmyCone _asbp_ship) 0 "/Game/StarterContent/Materials/M_CobbleStone_Smooth.M_CobbleStone_Smooth")
  (Default|Moveto _asbp_ship (+ (Math|Vector|MakeVector (.x _returnvalue) (.y _returnvalue) (.z _returnvalue)) "0.000000,0.000000,100.000000"))
  (return))

(fn GetWidgetReference
  (return (Variables|Actor|GetWidget)))