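; BP_Clock is a map clock Blueprint that can be started and stopped and exposes an elapsed-time value.
; While ClockOn is set, Tick accumulates delta seconds in CutTime, then moves whole seconds into TimeToIncrement and keeps the fractional remainder.
; RunClock and StopClock toggle counting, while setter and getter functions expose TimeElapsed.
; The Tick logic never adds TimeToIncrement to TimeElapsed.
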(event EventBeginPlay)

(event Collision|EventActorBeginOverlap
  (params (OtherActor :type Actor%20Object%20Reference)))

(event EventTick
  (params (DeltaSeconds :type Float%20%28single-precision%29))
  (if (Variables|Default|GetclockOn)
    (if (> (Variables|Default|GetcutTime) 1.0)
      (Variables|Default|SettimeToIncrement (Math|Float|Floor (Variables|Default|GetcutTime)))
      (Variables|Default|SetcutTime (- (Variables|Default|GetcutTime) (Variables|Default|GettimeToIncrement)))
      (else
        (Variables|Default|SetcutTime (+ (Variables|Default|GetcutTime) DeltaSeconds))))))

(fn ConstructionScript)

(fn SetTimeElapsed
  (params (timeElapsed :type Integer))
  (Variables|Default|SettimeElapsed timeElapsed))

(fn GetTimeElapsed
  (return (Variables|Default|GettimeElapsed)))

(fn RunClock
  (Variables|Default|SetclockOn true))

(fn StopClock
  (Variables|Default|SetclockOn false))