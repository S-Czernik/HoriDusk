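; Player ship for a planet-based map that travels between target positions, spending fuel and game time as it moves.
; BeginPlay adds the main UI and teleports the ship just above the tagged starting planet.
; MoveTo sets the target, and Tick moves toward it at constant speed, then snaps and flags Landed when close.
; While travelling, each frame advances BP_Clock and drains Fuel, so both costs depend on frame rate.
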(event EventBeginPlay
  ;[1 1 1] Default Position
  (bind _returnvalue (UserInterface|CreateWidget "/Game/mapAssets/BP_Main_UI.BP_Main_UI_C"))
  (UserInterface|Viewport|AddtoViewport _returnvalue 0)
  (bind _outactors (Actor|GetAllActorsOfClasswithTag "/Game/mapAssets/BP_Starting_Planet.BP_Starting_Planet_C" "StartingPlanet"))
  (for _array_element _outactors
    (Transformation|SetActorLocation (+ (Transformation|GetActorLocation _array_element) "0.000000,0.000000,100.000000") false true))
  (Variables|Default|SetTargetPosition (+ (Transformation|GetActorLocation _array_element) "0.000000,0.000000,100.000000")))

(event EventTick
  (params (DeltaSeconds :type Float%20%28single-precision%29))
  (bind _returnvalue (Transformation|GetActorLocation))
  ;[1 1 1] Calculate Position
  (if (Utilities|Operators|EqualEqual _returnvalue (Variables|Default|GetTargetPosition) 5e+01)
    (Transformation|SetActorLocation (Variables|Default|GetTargetPosition) false false)
    (Variables|Default|Setlanded true)
    (else
      (Variables|Default|Setlanded false)
      (Transformation|SetActorLocation (- _returnvalue (* (* (Math|Vector|Normalize (- _returnvalue (Variables|Default|GetTargetPosition))) DeltaSeconds) "500.000000,500.000000,500.000000")) false false)
      (bind _outactors (Actor|GetAllActorsOfClass "/Game/mapAssets/BP_Clock.BP_Clock_C"))
      (bind _newparam (Default|GetTimeElapsed _outactors))
      (Default|SetTimeElapsed _outactors (+ _newparam 80))
      (Variables|Default|SetFuel (- (Variables|Default|GetFuel) 1.0)))))

(fn ConstructionScript)

(fn Moveto
  (params (ToPosition :type Vector))
  (Variables|Default|SetTargetPosition ToPosition))