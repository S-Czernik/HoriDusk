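; BP_Target_Planet is a clickable planet that summons the nearest BP_Ship when selected.
; A click on its sphere resets every BP_Planet's material according to its "Target" tag, then sets Selected and gives this planet a cobblestone highlight.
; It then finds the closest ship, changes that ship's cone material and calls its MoveTo toward a point just above the planet.
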(event OnClicked(sphereComponent)
  (params (TouchedComponent :type Primitive%20Component%20Object%20Reference) (ButtonPressed :type Key%20Structure))
  (bind _returnvalue (Transformation|GetActorLocation))
  (bind _outactors (Actor|GetAllActorsOfClass "/Game/mapAssets/BP_Planet.BP_Planet_C"))
  (for _array_element _outactors
    (if (Actor|ActorHasTag _array_element "Target")
      (Rendering|Material|SetMaterial (Variables|/Game/mapAssets/BP_Planet.BP_Planet_C|GetsphereComponent _array_element) 0 "/Game/StarterContent/Materials/M_Water_Ocean.M_Water_Ocean")
      (else
        (Rendering|Material|SetMaterial (Variables|/Game/mapAssets/BP_Planet.BP_Planet_C|GetsphereComponent _array_element) 0 "/Game/StarterContent/Materials/M_Rock_Sandstone.M_Rock_Sandstone"))))
  (Variables|Default|Setselected true)
  (bind _outactors_2 (Actor|GetAllActorsOfClass "/Game/mapAssets/BP_Ship.BP_Ship_C"))
  (Rendering|Material|SetMaterial (Variables|Default|GetsphereComponent) 0 "/Game/StarterContent/Materials/M_CobbleStone_Smooth.M_CobbleStone_Smooth")
  (bind _asbp_ship (Utilities|Casting|CastToBP_Ship (.ReturnValue (Actor|FindNearestActor (Transformation|GetActorLocation self) _outactors_2))))
  (Rendering|Material|SetMaterial (Variables|/Game/mapAssets/BP_Ship.BP_Ship_C|GetmyCone _asbp_ship) 0 "/Game/StarterContent/Props/Materials/M_Bush.M_Bush")
  (Default|Moveto _asbp_ship (+ (Math|Vector|MakeVector (.x _returnvalue) (.y _returnvalue) (.z _returnvalue)) "0.000000,0.000000,100.000000")))

(event EventBeginPlay
  (Input|EnableInput (Game|GetPlayerController 0)))

(fn ConstructionScript)